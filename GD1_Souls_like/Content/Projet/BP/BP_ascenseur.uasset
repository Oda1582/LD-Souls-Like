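; Player-triggered elevator that lerps a slab between two editable positions, staying inactive until a one-time trigger enables it.
; The sphere overlap toggles travel direction, while top and bottom lever triggers call the slab to their end.
; Trajet and Retour timelines drive the movement, update arrival flags and animate both levers.
; The construction script derives play rate from speed over distance and places levers and triggers from variables.
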(event OnComponentBeginOverlap(TriggerLevierbas)
  (params (OverlappedComponent :type Primitive%20Component%20Object%20Reference) (OtherActor :type Actor%20Object%20Reference) (OtherComp :type Primitive%20Component%20Object%20Reference) (OtherBodyIndex :type Integer) (bFromSweep :type Boolean) (SweepResult :type Hit%20Result%20Structure%20%28by%20ref%29))
  (if (== OtherActor (Variables|Default|GetPlayer))
    (if (Variables|Default|GetPremière%20activation)
      (if (not (Variables|Default|GetArrivé%20en%20bas))
        (Components|Timeline|SetPlayRate (Variables|Default|GetTrajet) (Variables|Default|GetRate))
        (bind _deplacement (Timeline|Trajet PlayFromStart)
          (:Update
            (Transformation|SetRelativeLocation (Variables|Default|GetDalle) (Math|Vector|Lerp(Vector) (Variables|Default|GetPosition%20départ) (Variables|Default|GetPosition%20arrivé) _deplacement) false false)
            (Variables|Default|SetArrivé%20en%20bas true)
            (Variables|Default|SetArrivé%20en%20haut false)
            (Utilities|FlowControl|Sequence
              (:then_0
                (Components|MoveComponentTo (Variables|Default|GetST_Levier%20bas) "0, 0, 0" "-80.000000, 0, 0" false false 0.2 false))
              (:then_1
                (Components|MoveComponentTo (Variables|Default|GetST_Levier1%20haut) "0, 0, 0" "0, 0, 0" false false 0.2 false)))))))))

(event OnComponentEndOverlap(Sphere)
  (params (OverlappedComponent :type Primitive%20Component%20Object%20Reference) (OtherActor :type Actor%20Object%20Reference) (OtherComp :type Primitive%20Component%20Object%20Reference) (OtherBodyIndex :type Integer)))

(event OnComponentBeginOverlap(TriggerLevierhaut)
  (params (OverlappedComponent :type Primitive%20Component%20Object%20Reference) (OtherActor :type Actor%20Object%20Reference) (OtherComp :type Primitive%20Component%20Object%20Reference) (OtherBodyIndex :type Integer) (bFromSweep :type Boolean) (SweepResult :type Hit%20Result%20Structure%20%28by%20ref%29))
  (if (== OtherActor (Variables|Default|GetPlayer))
    (if (Variables|Default|GetPremière%20activation)
      (if (not (Variables|Default|GetArrivé%20en%20haut))
        (Components|Timeline|SetPlayRate (Variables|Default|GetRetour) (Variables|Default|GetRate))
        (bind _deplacement (Timeline|Retour ReverseFromEnd)
          (:Update
            (Transformation|SetRelativeLocation (Variables|Default|GetDalle) (Math|Vector|Lerp(Vector) (Variables|Default|GetPosition%20départ) (Variables|Default|GetPosition%20arrivé) _deplacement) false false)
            (Variables|Default|SetArrivé%20en%20bas false)
            (Variables|Default|SetArrivé%20en%20haut true)
            (Utilities|FlowControl|Sequence
              (:then_0
                (Components|MoveComponentTo (Variables|Default|GetST_Levier%20bas) "0, 0, 0" "0, 0, 0" false false 0.2 false))
              (:then_1
                (Components|MoveComponentTo (Variables|Default|GetST_Levier1%20haut) "0, 0, 0" "-80.000000, 0, 0" false false 0.2 false)))))))))

(event OnComponentBeginOverlap(Triggerfirsttime)
  (params (OverlappedComponent :type Primitive%20Component%20Object%20Reference) (OtherActor :type Actor%20Object%20Reference) (OtherComp :type Primitive%20Component%20Object%20Reference) (OtherBodyIndex :type Integer) (bFromSweep :type Boolean) (SweepResult :type Hit%20Result%20Structure%20%28by%20ref%29))
  (if (== OtherActor (Variables|Default|GetPlayer))
    (if (not (Variables|Default|GetStop%20reac))
      (Variables|Default|SetPremière%20activation true)
      (Transformation|SetRelativeRotation (Variables|Default|GetST_Levier1%20haut) (Variables|Default|GetRot%20levier%20haut) false false)
      (Transformation|SetRelativeRotation (Variables|Default|GetST_Levier%20bas) (Variables|Default|GetRot%20levier%20bas) false false)
      (Variables|Default|SetStop%20reac true))))

(event OnComponentBeginOverlap(Sphere)
  (params (OverlappedComponent :type Primitive%20Component%20Object%20Reference) (OtherActor :type Actor%20Object%20Reference) (OtherComp :type Primitive%20Component%20Object%20Reference) (OtherBodyIndex :type Integer) (bFromSweep :type Boolean) (SweepResult :type Hit%20Result%20Structure%20%28by%20ref%29))
  (if (== OtherActor (Variables|Default|GetPlayer))
    (if (Variables|Default|GetPremière%20activation)
      (if (Variables|Default|GetArrivé%20en%20bas)
        (if (not (Variables|Default|GetArrivé%20en%20haut))
          (Components|Timeline|SetPlayRate (Variables|Default|GetRetour) (Variables|Default|GetRate))
          (bind _deplacement (Timeline|Retour ReverseFromEnd)
            (:Update
              (Transformation|SetRelativeLocation (Variables|Default|GetDalle) (Math|Vector|Lerp(Vector) (Variables|Default|GetPosition%20départ) (Variables|Default|GetPosition%20arrivé) _deplacement) false false)
              (Variables|Default|SetArrivé%20en%20bas false)
              (Variables|Default|SetArrivé%20en%20haut true)
              (Utilities|FlowControl|Sequence
                (:then_0
                  (Components|MoveComponentTo (Variables|Default|GetST_Levier%20bas) "0, 0, 0" "0, 0, 0" false false 0.2 false))
                (:then_1
                  (Components|MoveComponentTo (Variables|Default|GetST_Levier1%20haut) "0, 0, 0" "-80.000000, 0, 0" false false 0.2 false))))))
        (else
          (Components|Timeline|SetPlayRate (Variables|Default|GetTrajet) (Variables|Default|GetRate))
          (bind _deplacement_2 (Timeline|Trajet PlayFromStart)
            (:Update
              (Transformation|SetRelativeLocation (Variables|Default|GetDalle) (Math|Vector|Lerp(Vector) (Variables|Default|GetPosition%20départ) (Variables|Default|GetPosition%20arrivé) _deplacement_2) false false)
              (Variables|Default|SetArrivé%20en%20bas true)
              (Variables|Default|SetArrivé%20en%20haut false)
              (Utilities|FlowControl|Sequence
                (:then_0
                  (Components|MoveComponentTo (Variables|Default|GetST_Levier%20bas) "0, 0, 0" "-80.000000, 0, 0" false false 0.2 false))
                (:then_1
                  (Components|MoveComponentTo (Variables|Default|GetST_Levier1%20haut) "0, 0, 0" "0, 0, 0" false false 0.2 false))))))))))

(event EventBeginPlay
  (Variables|Default|SetPlayer (Game|GetPlayerCharacter 0)))

(fn ConstructionScript
  (Variables|Default|SetRate (/ (Variables|Default|GetVitesse) (Math|Vector|Distance(Vector) (Variables|Default|GetPosition%20départ) (Variables|Default|GetPosition%20arrivé))))
  (Transformation|SetWorldLocationAndRotation (Variables|Default|GetSupport_levier_v2%20bas) (Variables|Default|GetLevier%20bas%20Pos) (Variables|Default|GetLevier%20bas%20Rotation) false false)
  (Components|Box|SetBoxExtent (Variables|Default|GetTrigger%20Levier%20bas) (Variables|Default|GetTaille%20Box%20trigger%20levier%20bas) true)
  (Transformation|SetRelativeLocationAndRotation (Variables|Default|GetTrigger%20Levier%20bas) (Variables|Default|GetPosition%20trigger%20levier%20bas) "0, 0, 0" false false)
  (Transformation|SetWorldLocationAndRotation (Variables|Default|GetSupport_levier_v3%20haut) (Variables|Default|GetLevier%20haut%20pos) (Variables|Default|GetLevier%20haut%20rot) false false)
  (Components|Box|SetBoxExtent (Variables|Default|GetTrigger%20Levier%20haut) (Variables|Default|GetTaille%20box%20trivver%20levier%20haut) true)
  (Transformation|SetRelativeLocationAndRotation (Variables|Default|GetTrigger%20Levier%20haut) (Variables|Default|GetPosition%20trigger%20levier%20haut) "0, 0, 0" false false)
  (Transformation|SetWorldLocationAndRotation (Variables|Default|GetTrigger%20first%20time) (Variables|Default|GetTrigger%20first%20pos) (Variables|Default|GetTrigger%20first%20rot) false false)
  (Components|Box|SetBoxExtent (Variables|Default|GetTrigger%20first%20time) (Variables|Default|GetTrigger%20first%20taille) true))