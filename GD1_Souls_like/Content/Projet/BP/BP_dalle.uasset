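; Moving slab (dalle) Blueprint that slides a component between a start and an end relative position.
; The construction script divides Vitesse by the distance between both points to get a play rate, so travel speed can stay independent of path length.
; On BeginPlay, the Trajet timeline plays at that rate and drives a position lerp without sweep.
; Trigger overlap events check for the player but perform no action.
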(event OnComponentBeginOverlap(Trigger)
  (params (OverlappedComponent :type Primitive%20Component%20Object%20Reference) (OtherActor :type Actor%20Object%20Reference) (OtherComp :type Primitive%20Component%20Object%20Reference) (OtherBodyIndex :type Integer) (bFromSweep :type Boolean) (SweepResult :type Hit%20Result%20Structure%20%28by%20ref%29))
  (if (== OtherActor (Variables|Default|GetPlayer))
    _))

(event OnComponentEndOverlap(Trigger)
  (params (OverlappedComponent :type Primitive%20Component%20Object%20Reference) (OtherActor :type Actor%20Object%20Reference) (OtherComp :type Primitive%20Component%20Object%20Reference) (OtherBodyIndex :type Integer))
  (if (== (Variables|Default|GetPlayer) OtherActor)
    _))

(event EventBeginPlay
  (Variables|Default|SetPlayer (Game|GetPlayerCharacter 0))
  (Components|Timeline|SetPlayRate (Variables|Default|GetTrajet) (Variables|Default|GetRate))
  (bind _deplacement (Timeline|Trajet Play)
    (:Update
      (Transformation|SetRelativeLocation (Variables|Default|GetDalle) (Math|Vector|Lerp(Vector) (Variables|Default|GetPosition%20départ) (Variables|Default|GetPosition%20arrivé) _deplacement) false false))))

(fn ConstructionScript
  (Variables|Default|SetRate (/ (Variables|Default|GetVitesse) (Math|Vector|Distance(Vector) (Variables|Default|GetPosition%20départ) (Variables|Default|GetPosition%20arrivé)))))