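; BP_Light is a configurable light actor with a point light component.
; Its construction script applies the actor's intensity, relative position and attenuation radius variables to the point light.
; The event graph has no active logic, and a spot light intensity call is left unconnected, so it never runs.
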(event EventBeginPlay)

(event Collision|EventActorBeginOverlap
  (params (OtherActor :type Actor%20Object%20Reference)))

(event EventTick
  (params (DeltaSeconds :type Float%20%28single-precision%29)))

(fn ConstructionScript
  (Rendering|Components|Light|SetIntensity (Variables|Default|GetPointLight) (Variables|Default|Getintensity%20point%20light))
  (Transformation|SetRelativeLocationAndRotation (Variables|Default|GetPointLight) (Variables|Default|GetPoint%20light%20pos) "0, 0, 0" false false)
  (Rendering|Lighting|SetAttenuationRadius (Variables|Default|GetPointLight) (Variables|Default|GetPoint%20light%20attenuation%20radius)))