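; Respawn actor that teleports the player to a bonfire checkpoint's respawn location when they enter the Death box.
; Four bonfire boxes set Bon flags and clear lower-numbered ones, each firing once via its Stop flag, so the most recently activated checkpoint wins.
; The construction script sizes all trigger boxes and places the bonfires in world space from variables.
; Death does nothing until a bonfire flag is set.
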(event OnComponentBeginOverlap(Death)
  (params (OverlappedComponent :type Primitive%20Component%20Object%20Reference) (OtherActor :type Actor%20Object%20Reference) (OtherComp :type Primitive%20Component%20Object%20Reference) (OtherBodyIndex :type Integer) (bFromSweep :type Boolean) (SweepResult :type Hit%20Result%20Structure%20%28by%20ref%29))
  (if (== OtherActor (Variables|Default|GetPlayer))
    (if (Variables|Default|GetBon%201)
      (Transformation|Teleport (Variables|Default|GetPlayer) (Variables|Default|GetDeath%20loc%201) (Variables|Default|GetDest%20Rotation))
      (elif (Variables|Default|GetBon%202)
        (Transformation|Teleport (Variables|Default|GetPlayer) (Variables|Default|GetDeath%20loc%202) "0, 0, 0")
        (elif (Variables|Default|GetBon%203)
          (Transformation|Teleport (Variables|Default|GetPlayer) (Variables|Default|GetDeath%20loc%203) "0, 0, 0")
          (elif (Variables|Default|GetBon%204)
            (Transformation|Teleport (Variables|Default|GetPlayer) (Variables|Default|GetDeath%20loc%204) "0, 0, 0")))))))

(event OnComponentBeginOverlap(Bonfire1)
  (params (OverlappedComponent :type Primitive%20Component%20Object%20Reference) (OtherActor :type Actor%20Object%20Reference) (OtherComp :type Primitive%20Component%20Object%20Reference) (OtherBodyIndex :type Integer) (bFromSweep :type Boolean) (SweepResult :type Hit%20Result%20Structure%20%28by%20ref%29))
  (if (== OtherActor (Variables|Default|GetPlayer))
    (if (Variables|Default|GetStop%201)
      (Variables|Default|SetBon%201 true)
      (Variables|Default|SetStop%201 false))))

(event OnComponentBeginOverlap(Bonfire2)
  (params (OverlappedComponent :type Primitive%20Component%20Object%20Reference) (OtherActor :type Actor%20Object%20Reference) (OtherComp :type Primitive%20Component%20Object%20Reference) (OtherBodyIndex :type Integer) (bFromSweep :type Boolean) (SweepResult :type Hit%20Result%20Structure%20%28by%20ref%29))
  (if (== OtherActor (Variables|Default|GetPlayer))
    (if (Variables|Default|GetStop%202)
      (Variables|Default|SetBon%201 false)
      (Variables|Default|SetBon%202 true)
      (Variables|Default|SetStop%202 false))))

(event OnComponentBeginOverlap(Bonfire3)
  (params (OverlappedComponent :type Primitive%20Component%20Object%20Reference) (OtherActor :type Actor%20Object%20Reference) (OtherComp :type Primitive%20Component%20Object%20Reference) (OtherBodyIndex :type Integer) (bFromSweep :type Boolean) (SweepResult :type Hit%20Result%20Structure%20%28by%20ref%29))
  (if (== OtherActor (Variables|Default|GetPlayer))
    (if (Variables|Default|GetStop%203)
      (Variables|Default|SetBon%201 false)
      (Variables|Default|SetBon%202 false)
      (Variables|Default|SetBon%203 true)
      (Variables|Default|SetStop%203 false))))

(event OnComponentBeginOverlap(Bonfire4)
  (params (OverlappedComponent :type Primitive%20Component%20Object%20Reference) (OtherActor :type Actor%20Object%20Reference) (OtherComp :type Primitive%20Component%20Object%20Reference) (OtherBodyIndex :type Integer) (bFromSweep :type Boolean) (SweepResult :type Hit%20Result%20Structure%20%28by%20ref%29))
  (if (== OtherActor (Variables|Default|GetPlayer))
    (if (Variables|Default|GetStop%204)
      (Variables|Default|SetBon%201 false)
      (Variables|Default|SetBon%202 false)
      (Variables|Default|SetBon%203 false)
      (Variables|Default|SetBon%204 true)
      (Variables|Default|SetStop%204 false))))

(event EventBeginPlay
  (Variables|Default|SetPlayer (Game|GetPlayerCharacter 0)))

(fn ConstructionScript
  (Components|Box|SetBoxExtent (Variables|Default|GetDeath) (Variables|Default|GetIn%20Box%20Extent) true)
  (Components|Box|SetBoxExtent (Variables|Default|GetBonfire%201) (Variables|Default|GetBon%20pos%201%20) true)
  (Components|Box|SetBoxExtent (Variables|Default|GetBonfire%202) (Variables|Default|GetBon%20pos%202) true)
  (Components|Box|SetBoxExtent (Variables|Default|GetBonfire%203) (Variables|Default|GetBon%20pos%203) true)
  (Components|Box|SetBoxExtent (Variables|Default|GetBonfire%204) (Variables|Default|GetBon%20pos%204) true)
  (Transformation|SetWorldLocationAndRotation (Variables|Default|GetBonfire%201) (Variables|Default|GetBonloc%201) (Variables|Default|GetBonrot%201) false false)
  (Transformation|SetWorldLocationAndRotation (Variables|Default|GetBonfire%202) (Variables|Default|GetBonloc%202) (Variables|Default|GetBonrot%202) false false)
  (Transformation|SetWorldLocationAndRotation (Variables|Default|GetBonfire%203) (Variables|Default|GetBonloc%203) (Variables|Default|GetBonrot%203) false false)
  (Transformation|SetWorldLocationAndRotation (Variables|Default|GetBonfire%204) (Variables|Default|GetBonloc%204) (Variables|Default|GetBonrot%204) false false))